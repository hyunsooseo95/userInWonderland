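; BP_Door_Red is a lockable door actor that opens or closes when a player holding the matching key interacts with it.
; OnInteraction checks that the player is valid and has the key for the door's KeyChannel, then toggles between Open and Close based on the Open flag.
; A RotateDoorTimeline drives the Door component's relative yaw, playing forward to open and in reverse to close.
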(event Custom|Open
  (Variables|Private|SetOpen? true)
  (bind _doorrotation (Timeline|RotateDoor%20Timeline Play)
    (:Update
      (Transformation|SetRelativeRotation (Variables|Default|GetDoor) (Math|Rotator|MakeRotator 0.0 0.0 _doorrotation) false false))))

(event Custom|close
  (Variables|Private|SetOpen? false)
  (bind _doorrotation (Timeline|RotateDoor%20Timeline Reverse)
    (:Update
      (Transformation|SetRelativeRotation (Variables|Default|GetDoor) (Math|Rotator|MakeRotator 0.0 0.0 _doorrotation) false false))))

(event EventBeginPlay)

(event Collision|EventActorBeginOverlap
  (params (OtherActor :type Actor%20Object%20Reference)))

(event EventTick
  (params (DeltaSeconds :type Float%20%28single-precision%29)))

(event EventOnInteraction
  (params (Player :type Vive%20Pawn%20Character%20Object%20Reference))
  (Utilities|IsValid Player
    (:Is%20Valid
      (if (Default|HasKey? Player (Variables|Constants|GetKeyChannel))
        (if (Variables|Private|GetOpen?)
          (CallFunction|Close)
          (else
            (CallFunction|Open)))))))

(fn ConstructionScript)