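; Enemy rabbit Blueprint that chases the VR player pawn while it overlaps the actor and attacks on reaching it.
; AI MoveTo success plays an attack montage gated by an AttackRate cooldown, then re-chases if the player remains in range.
; Ending overlap stops movement; any damage plays a shrink montage and destroys the rabbit after a short delay.
; The Trigger component's overlap handler has no effect.
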(event OnComponentBeginOverlap(Trigger)
  (params (OverlappedComponent :type Primitive%20Component%20Object%20Reference) (OtherActor :type Actor%20Object%20Reference) (OtherComp :type Primitive%20Component%20Object%20Reference) (OtherBodyIndex :type Integer) (bFromSweep :type Boolean) (SweepResult :type Hit%20Result%20Structure%20%28by%20ref%29))
  (if (== OtherActor 0)
    _))

(event Custom|Chase%20The%20Player
  (AI|AIMoveTo self "0, 0, 0" (Game|GetPlayerCharacter 0) 1e+02 false
    (:OnSuccess
      (if (Variables|Default|GetCan%20Attack)
        (Variables|Default|SetCan%20Attack false)
        (Animation|Montage|PlayMontage (Variables|Character|GetMesh) "/Game/Assets/Rabbit_temp/enemy_rabbit_attack.enemy_rabbit_attack"
          (:then
            (Utilities|FlowControl|Delay (Variables|Default|GetAttack%20Rate))
            (Variables|Default|SetCan%20Attack true))
          (:OnCompleted
            (if (Variables|Default|GetPlayer%20in%20Range)
              (CallFunction|ChasethePlayer))))
        (else
          (CallFunction|ChasethePlayer))))))

(event Game|Damage|EventAnyDamage
  (params (Damage :type Float%20%28single-precision%29) (DamageType :type Damage%20Type%20Object%20Reference) (InstigatedBy :type Controller%20Object%20Reference) (DamageCauser :type Actor%20Object%20Reference))
  (if true
    (Components|Animation|SetAnimationMode (Variables|Character|GetMesh) "AnimationBlueprint")
    (Animation|Montage|PlayMontage (Variables|Character|GetMesh) "/Game/Assets/Rabbit_temp/enemy_rabbit_shrink.enemy_rabbit_shrink"
      (:then
        (Utilities|FlowControl|Delay 0.7)
        (Actor|DestroyActor)))))

(event Collision|EventActorBeginOverlap
  (params (OtherActor :type Actor%20Object%20Reference))
  (Utilities|Casting|CastToVive_PawnCharacter OtherActor)
  (Variables|Default|SetPlayer%20in%20Range true)
  (CallFunction|ChasethePlayer))

(event Collision|EventActorEndOverlap
  (params (OtherActor :type Actor%20Object%20Reference))
  (Utilities|Casting|CastToVive_PawnCharacter OtherActor)
  (Variables|Default|SetPlayer%20in%20Range false)
  (Development|PrintString "Player Excaped")
  (Components|Movement|StopMovementImmediately (Variables|Character|GetCharacterMovement)))

(fn ConstructionScript)