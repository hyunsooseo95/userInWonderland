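; Enemy rabbit AI character that chases and attacks the player when a Vive pawn character overlaps it.
; Overlap begin starts an AI MoveTo toward player 0, while overlap end clears the in-range flag and stops movement.
; On arrival it plays a montage, gated by an attack-rate cooldown, and chases again on completion if still in range.
; During cooldown it re-issues the chase without checking range; no damage is applied here.
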(event Custom|Chase%20The%20Player
  (AI|AIMoveTo self "0, 0, 0" (Game|GetPlayerCharacter 0) 1e+02 false
    (:OnSuccess
      (if (Variables|Default|GetCan%20Attack)
        (Variables|Default|SetCan%20Attack false)
        (Animation|Montage|PlayMontage (Variables|Character|GetMesh) 0
          (:then
            (Utilities|FlowControl|Delay (Variables|Default|GetAttack%20Rate))
            (Variables|Default|SetCan%20Attack true))
          (:OnCompleted
            (if (Variables|Default|GetPlayer%20in%20Range)
              (CallFunction|ChasethePlayer))))
        (else
          (CallFunction|ChasethePlayer))))))

(event Collision|EventActorBeginOverlap
  (params (OtherActor :type Actor%20Object%20Reference))
  (Utilities|Casting|CastToVive_PawnCharacter OtherActor)
  (Variables|Default|SetPlayer%20in%20Range true)
  (CallFunction|ChasethePlayer))

(event Collision|EventActorEndOverlap
  (params (OtherActor :type Actor%20Object%20Reference))
  (Utilities|Casting|CastToVive_PawnCharacter OtherActor)
  (Variables|Default|SetPlayer%20in%20Range false)
  (Development|PrintString "Player Excaped")
  (Components|Movement|StopMovementImmediately (Variables|Character|GetCharacterMovement)))

(fn ConstructionScript)